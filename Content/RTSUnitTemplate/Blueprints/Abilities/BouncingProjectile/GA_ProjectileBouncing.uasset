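; Gameplay ability for RTS units that casts a homing, bouncing projectile at the unit being chased.
; Activation puts the unit into the Casting state with a tinted cast bar and a cast time shortened by spent ability points.
; On cast completion it plays a montage and, if the commit succeeds, spawns the multi-pierce projectile, applies a cooldown effect and ends; a failed commit just ends.
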(event `self.K2_ActivateAbility`
  (bind _asunit_base (cast `UnitBase` (`self.GetAvatarActorFromActorInfo`)))
  (`KismetSystemLibrary.PrintString` "START CASTING")
  (`UnitBase.SetTimerWidgetCastingColor` _asunit_base (struct :`R` 0.939012 :`G` 0.012392 :`B` 1.0 :`A` 1.0))
  (set `UnitBase.UnitControlTimer` 0.0 _asunit_base)
  (bind _output_get (set `self.CastTime` 2.5))
  (bind (_leveldata_experience _leveldata_characterlevel _leveldata_talentpoints _leveldata_usedtalentpoints _leveldata_abilitypoints _leveldata_usedabilitypoints _leveldata_usedabilitypointsarray) (break `LevelData` (`LevelUnit.LevelData` _asunit_base)))
  (set `UnitBase.CastTime` (- _output_get (* (`KismetMathLibrary.Conv_IntToDouble` (`|GetArrayItem` _leveldata_usedabilitypointsarray 3)) 0.3)) _asunit_base)
  (`AbilityUnit.SetUnitState` _asunit_base "Casting"))

(event `self.K2_OnEndAbility`
  (params (bWasCancelled :type Boolean)))

(event `self.OnAbilityCastComplete`
  (bind (_returnvalue_owneractor _returnvalue_avataractor _returnvalue_playercontroller _returnvalue_abilitysystemcomponent _returnvalue_skeletalmeshcomponent) (break `GameplayAbilityActorInfo` (`self.GetActorInfo`)))
  (`KismetSystemLibrary.PrintString` "CAST COMPLETED!!!!!!!!!!!!!!!!!!!")
  (`|PlayMontage` _returnvalue_skeletalmeshcomponent "/Game/ControlRig/Characters/Mannequins/Animations/Manny/Manny_Test_Montage.Manny_Test_Montage"
    (:`then`
      (bind _asunit_base (cast `UnitBase` (`self.GetAvatarActorFromActorInfo`)))
      (bind _returnvalue (`self.K2_CommitAbility`))
      (if _returnvalue
        (`UnitBase.SpawnProjectileFromClass` _asunit_base (`UnitBase.UnitToChase` _asunit_base) _asunit_base "/RTSUnitTemplate/RTSUnitTemplate/Blueprints/Abilities/Projectile/BP_Projectile_5.BP_Projectile_5_C" 4 true 1 0.0 true false true 0.0 2.0)
        (`self.BP_ApplyGameplayEffectToOwner` "/RTSUnitTemplate/RTSUnitTemplate/Blueprints/Abilities/Projectile/GE_Projectile_Cooldown.GE_Projectile_Cooldown_C")
        (`self.K2_EndAbility`)
        (else
          (`self.K2_EndAbility`))))))