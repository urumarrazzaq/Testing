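; Gameplay ability for RTS units that fires a single homing projectile at the unit's current chase target, set to bounce back.
; On activation it casts the avatar to UnitBase, commits the ability, spawns BP_Projectile_5 with follow, pierce and bounce-back options, then ends.
; Montage playback, debug prints and manual cooldown-effect application remain as disconnected nodes and never run.
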(event `self.K2_ActivateAbility`
  (bind _asunit_base (cast `UnitBase` (`self.GetAvatarActorFromActorInfo`)))
  (bind _returnvalue (`self.K2_CommitAbility`))
  (if _returnvalue
    (`UnitBase.SpawnProjectileFromClass` _asunit_base (`UnitBase.UnitToChase` _asunit_base) _asunit_base "/RTSUnitTemplate/RTSUnitTemplate/Blueprints/Abilities/Projectile/BP_Projectile_5.BP_Projectile_5_C" 4 true 1 0.0 false true true 0.0 1.0)
    (`self.K2_EndAbility`)
    (else
      (`self.K2_EndAbility`))))