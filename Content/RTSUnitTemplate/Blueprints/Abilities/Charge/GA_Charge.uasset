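; Gameplay ability that makes an RTS unit charge at the unit it is chasing.
; On activation it casts the avatar to UnitBase and, if UnitToChase is valid, commits the ability.
; It then calls StartAcceleratingTowardsDestination toward the target's current location with a horizontal velocity, and ends immediately.
; Debug prints, montage playback and manual cooldown application are disconnected.
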(event `self.K2_ActivateAbility`
  (bind _asunit_base (cast `UnitBase` (`self.GetAvatarActorFromActorInfo`)))
  (bind _unittochase (`UnitBase.UnitToChase` _asunit_base))
  (if (`KismetSystemLibrary.IsValid` _unittochase)
    (bind _returnvalue (`self.K2_CommitAbility`))
    (if _returnvalue
      (bind _returnvalue_2 (`Actor.K2_GetActorLocation` _unittochase))
      (`UnitBase.StartAcceleratingTowardsDestination` _asunit_base _returnvalue_2 (* (`KismetMathLibrary.Normal` (- _returnvalue_2 (`Actor.K2_GetActorLocation` _asunit_base))) (5000.0 5000.0 0.0)) 20.0 2000.0)
      (`self.K2_EndAbility`)
      (else
        (`self.K2_EndAbility`)))))