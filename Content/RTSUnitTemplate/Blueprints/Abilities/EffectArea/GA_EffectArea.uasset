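; Gameplay ability that lets an RTS unit drop a scaled-up damage effect area on the unit it is chasing.
; It plays a montage and, only on completion, commits the ability and has player controller 0 spawn BP_EffectArea_Dmg for the caster's team, slightly below the target's position.
; An interrupted montage or failed unit cast never reaches EndAbility, and the chase target is not validity-checked.
; The manual cooldown-effect node is disconnected.
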(event `self.K2_ActivateAbility`
  (bind (_returnvalue_owneractor _returnvalue_avataractor _returnvalue_playercontroller _returnvalue_abilitysystemcomponent _returnvalue_skeletalmeshcomponent) (break `GameplayAbilityActorInfo` (`self.GetActorInfo`)))
  (`|PlayMontage` _returnvalue_skeletalmeshcomponent "/Game/ControlRig/Characters/Mannequins/Animations/Manny/Manny_Test_Montage.Manny_Test_Montage"
    (:`OnCompleted`
      (bind _asunit_base (cast `UnitBase` (`self.GetAvatarActorFromActorInfo`)))
      (bind _ascontroller_base (cast `ControllerBase` (`GameplayStatics.GetPlayerController` 0))
        (:`then`
          (bind _returnvalue (`self.K2_CommitAbility`))
          (if _returnvalue
            (`ControllerBase.SpawnEffectArea` _ascontroller_base (`UnitBase.TeamId` _asunit_base) (- (`Actor.K2_GetActorLocation` (`UnitBase.UnitToChase` _asunit_base)) (0.0 0.0 60.0)) (3.0 3.0 3.0) "/RTSUnitTemplate/RTSUnitTemplate/Blueprints/Actors/Effects/BP_EffectArea_Dmg.BP_EffectArea_Dmg_C" null)
            (`self.K2_EndAbility`)
            (else
              (`self.K2_EndAbility` :!label _label))))
        (:`CastFailed`
          (goto _label))))))