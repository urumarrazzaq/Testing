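; Gameplay ability from the RTS unit template that lets a unit start a paid building construction.
; On activation it asks the ResourceGameMode whether the unit's team can afford a hardcoded primary-resource cost.
; If so, the unit spawns a replicated BP_WorkArea_BuildArea flagged as paid; otherwise debug text prints and an error sound plays.
; The cast-complete event is empty and EndAbility is left unwired, so the graph never ends the ability.
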(event `self.K2_ActivateAbility`
  (bind _asunit_base (cast `UnitBase` (`self.GetAvatarActorFromActorInfo`)))
  (bind _asresource_game_mode (cast `ResourceGameMode` (`GameplayStatics.GetGameMode`)))
  (`KismetSystemLibrary.PrintString` "Found GameMode")
  (if (`ResourceGameMode.CanAffordConstruction` _asresource_game_mode (make `BuildingCost` 100) (`SpawnerUnit.TeamId` _asunit_base))
    (`KismetSystemLibrary.PrintString` "Trying Spawn WorkArea")
    (`WorkingUnitBase.SpawnWorkAreaReplicated` _asunit_base "/RTSUnitTemplate/RTSUnitTemplate/Blueprints/Actors/Worker/BP_WorkArea_BuildArea.BP_WorkArea_BuildArea_C" null true)
    (else
      (`KismetSystemLibrary.PrintString` (`KismetStringLibrary.Conv_DoubleToString` 0.0))
      (`KismetSystemLibrary.PrintString` "IS NOT ENOUGH MONEY")
      (`GameplayStatics.PlaySound2D` "/Engine/EditorSounds/Notifications/CompileFailed_Cue.CompileFailed_Cue" 1.0 1.0 0.0 null null))))

(event `self.OnAbilityCastComplete`)