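; Gameplay ability that lets an RTS unit start placing the third building type by spawning its build work area.
; On activation it reads the team's Primary resource from ResourceGameMode and, if the cost threshold is met, calls the unit's replicated work-area spawn.
; Otherwise it prints debug text and plays a failure sound.
; The graph only checks the resource without deducting it, and its EndAbility call is unconnected.
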(event `self.K2_ActivateAbility`
  (bind _asunit_base (cast `UnitBase` (`self.GetAvatarActorFromActorInfo`)))
  (bind _asresource_game_mode (cast `ResourceGameMode` (`GameplayStatics.GetGameMode`)))
  (bind _returnvalue (`ResourceGameMode.GetResource` _asresource_game_mode (`SpawnerUnit.TeamId` _asunit_base) "Primary"))
  (`KismetSystemLibrary.PrintString` "Found GameMode")
  (if (>= _returnvalue 100.0)
    (`KismetSystemLibrary.PrintString` "Trying Spawn WorkArea")
    (`WorkingUnitBase.SpawnWorkAreaReplicated` _asunit_base "/RTSUnitTemplate/RTSUnitTemplate/Blueprints/Actors/Worker/BP_WorkArea_BuildArea3.BP_WorkArea_BuildArea3_C" null)
    (else
      (`KismetSystemLibrary.PrintString` (`KismetStringLibrary.Conv_DoubleToString` _returnvalue))
      (`KismetSystemLibrary.PrintString` "IS NOT ENOUGH MONEY")
      (`GameplayStatics.PlaySound2D` "/Engine/EditorSounds/Notifications/CompileFailed_Cue.CompileFailed_Cue" 1.0 1.0 0.0 null null))))

(event `self.OnAbilityCastComplete`)